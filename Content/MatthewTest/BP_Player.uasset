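; BP_Player is a test player character with basic movement, look and jump driven by Enhanced Input.
; BeginPlay casts player controller 0 to BP_PlayerController and adds the IMC_CharacterMovement mapping context.
; Four separate walk actions add movement scaled by Speed along control-rotation directions with pitch zeroed, so looking up or down does not tilt movement.
; The look action drives controller yaw and inverted pitch, and the jump action calls Jump.
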(event `EnhancedInput|/Game/MatthewTest/IA_Jump`
  (params (ActionValue :type Boolean) (ElapsedSeconds :type "Float (double-precision)") (TriggeredSeconds :type "Float (double-precision)") (InputAction :type "InputAction Object Reference" :default "/Game/MatthewTest/IA_Jump.IA_Jump"))
  ; Simple Movement
  (:`Triggered`
    (`self.Jump`)))

(event `self.ReceiveBeginPlay`
  (bind _asbp_player_controller (cast `/Game/MatthewTest/BP_PlayerController` (`GameplayStatics.GetPlayerController` 0)))
  (`EnhancedInputSubsystemInterface.AddMappingContext` (pcsubsystem `EnhancedInputLocalPlayerSubsystem` _asbp_player_controller) "/Game/MatthewTest/IMC_CharacterMovement.IMC_CharacterMovement" 0 (make `ModifyContextOptions` false)))

(event `EnhancedInput|/Game/MatthewTest/IA_Look`
  (params (ActionValue :type "Vector2D Structure") (ElapsedSeconds :type "Float (double-precision)") (TriggeredSeconds :type "Float (double-precision)") (InputAction :type "InputAction Object Reference" :default "/Game/MatthewTest/IA_Look.IA_Look"))
  ; Simple Movement
  (:`Triggered`
    (`self.AddControllerYawInput` ActionValue_X)
    (`self.AddControllerPitchInput` (* ActionValue_Y -1.0))))

(event `EnhancedInput|/Game/MatthewTest/IA_WalkBackward`
  (params (ActionValue :type Boolean) (ElapsedSeconds :type "Float (double-precision)") (TriggeredSeconds :type "Float (double-precision)") (InputAction :type "InputAction Object Reference" :default "/Game/MatthewTest/IA_WalkBackward.IA_WalkBackward"))
  (bind (_returnvalue_roll _returnvalue_pitch _returnvalue_yaw) (`KismetMathLibrary.BreakRotator` (`self.GetControlRotation`)))
  ; Simple Movement
  (:`Triggered`
    (`self.AddMovementInput` (`KismetMathLibrary.Normal` (`KismetMathLibrary.GetForwardVector` (`KismetMathLibrary.MakeRotator` _returnvalue_roll 0.0 _returnvalue_yaw))) (* (`self.Speed`) -1.0))))

(event `EnhancedInput|/Game/MatthewTest/IA_WalkForward`
  (params (ActionValue :type Boolean) (ElapsedSeconds :type "Float (double-precision)") (TriggeredSeconds :type "Float (double-precision)") (InputAction :type "InputAction Object Reference" :default "/Game/MatthewTest/IA_WalkForward.IA_WalkForward"))
  (bind (_returnvalue_roll _returnvalue_pitch _returnvalue_yaw) (`KismetMathLibrary.BreakRotator` (`self.GetControlRotation`)))
  ; Simple Movement
  (:`Triggered`
    (`self.AddMovementInput` (`KismetMathLibrary.Normal` (`KismetMathLibrary.GetForwardVector` (`KismetMathLibrary.MakeRotator` _returnvalue_roll 0.0 _returnvalue_yaw))) (`self.Speed`))))

(event `EnhancedInput|/Game/MatthewTest/IA_WalkRight`
  (params (ActionValue :type Boolean) (ElapsedSeconds :type "Float (double-precision)") (TriggeredSeconds :type "Float (double-precision)") (InputAction :type "InputAction Object Reference" :default "/Game/MatthewTest/IA_WalkRight.IA_WalkRight"))
  (bind (_returnvalue_roll _returnvalue_pitch _returnvalue_yaw) (`KismetMathLibrary.BreakRotator` (`self.GetControlRotation`)))
  ; Simple Movement
  (:`Triggered`
    (`self.AddMovementInput` (`KismetMathLibrary.Normal` (`KismetMathLibrary.GetRightVector` (`KismetMathLibrary.MakeRotator` 0.0 0.0 _returnvalue_yaw))) (`self.Speed`))))

(event `EnhancedInput|/Game/MatthewTest/IA_WalkLeft`
  (params (ActionValue :type Boolean) (ElapsedSeconds :type "Float (double-precision)") (TriggeredSeconds :type "Float (double-precision)") (InputAction :type "InputAction Object Reference" :default "/Game/MatthewTest/IA_WalkLeft.IA_WalkLeft"))
  (bind (_returnvalue_roll _returnvalue_pitch _returnvalue_yaw) (`KismetMathLibrary.BreakRotator` (`self.GetControlRotation`)))
  ; Simple Movement
  (:`Triggered`
    (`self.AddMovementInput` (`KismetMathLibrary.Normal` (`KismetMathLibrary.GetRightVector` (`KismetMathLibrary.MakeRotator` 0.0 0.0 _returnvalue_yaw))) (* (`self.Speed`) -1.0))))

(fn `UserConstructionScript`)