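; BP_Laptop is an interactable laptop that pulls the player's camera in to show a usable screen UI.
; Interact removes the movement mapping context, then a timeline scaled by CameraMoveTime lerps the player camera to CameraLocation, facing CameraViewSpot.
; When the move finishes, it creates UW_LaptopScreen on the Screen widget component, shows the cursor and adds the laptop mapping context.
; SetScreen swaps in any widget class and focuses it with Game and UI input.
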(event `SetScreen`
  (params (NewScreen :type "UserWidget Class Reference"))
  (bind _returnvalue (`|CreateWidget` NewScreen))
  (`WidgetComponent.SetWidget` (`self.Screen`) _returnvalue)
  (bind _output_get (set `self.CurWidget` _returnvalue))
  (`WidgetBlueprintLibrary.SetInputMode_GameAndUIEx` (`/Game/MatthewTest/Player/BP_Player.PlayerController` (stale `/Game/Structure/IE_Interactable.Interact` _asbp_player)) _output_get "DoNotLock" false))

(event `/Game/Structure/IE_Interactable.Interact`
  (bind _returnvalue (`SceneComponent.K2_GetComponentLocation` (`self.CameraLocation`)))
  (bind _asbp_player (cast `/Game/MatthewTest/Player/BP_Player` (`GameplayStatics.GetPlayerCharacter` 0)))
  (bind _playercontroller (`/Game/MatthewTest/Player/BP_Player.PlayerController` _asbp_player))
  (bind _returnvalue_2 (pcsubsystem `EnhancedInputLocalPlayerSubsystem` _playercontroller))
  ; Makes player unable to move, adds inputs for while in laptop (Leave, confirm purchase etc.)
  (`EnhancedInputSubsystemInterface.RemoveMappingContext` _returnvalue_2 "/Game/MatthewTest/Player/IMC_CharacterMovement.IMC_CharacterMovement" (make `ModifyContextOptions` true))
  (`EnhancedInputLibrary.FlushPlayerInput` _playercontroller)
  (bind _camera (`/Game/MatthewTest/Player/BP_Player.Camera` _asbp_player))
  (set `self.OriginalCamRotation` (`SceneComponent.K2_GetComponentRotation` _camera))
  ; Can make swoop in take more or less time
  (set `CameraComponent.bUsePawnControlRotation` false _camera)
  (`TimelineComponent.SetPlayRate` (`self.CameraMovement`) (/ 1.0 (`self.CameraMoveTime`)))
  (bind (_direction _newtrack_0) (`Timeline|CameraMovement` :!via `PlayFromStart`)
    (:`Update`
      (`SceneComponent.K2_SetWorldLocationAndRotation` _camera (`KismetMathLibrary.VLerp` (`SceneComponent.K2_GetComponentLocation` (`/Game/MatthewTest/Player/BP_Player.CameraDefaultLocation` _asbp_player)) _returnvalue _newtrack_0) (`KismetMathLibrary.RLerp` (`self.OriginalCamRotation`) (`KismetMathLibrary.FindLookAtRotation` _returnvalue (`SceneComponent.K2_GetComponentLocation` (`self.CameraViewSpot`))) _newtrack_0) false false))
    (:`Finished`
      (`self.SetScreen` "/Game/MatthewTest/Interactables/UW_LaptopScreen.UW_LaptopScreen_C")
      (set `PlayerController.bShowMouseCursor` true _playercontroller)
      (`EnhancedInputSubsystemInterface.AddMappingContext` _returnvalue_2 "/Game/MatthewTest/Player/IMC_Laptop.IMC_Laptop" 0 (struct)))))

(fn `UserConstructionScript`
  (`parent.UserConstructionScript`))