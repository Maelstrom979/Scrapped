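; Base interactable shelf that moves the player's camera into a slot-by-slot shelving view.
; BeginPlay registers "Items"-tagged scene components as slots and attaches offset look and camera points to each.
; Interact swaps player input to IMC_Shelving, timeline-lerps the camera to the first slot and opens UW_Shelf.
; LookLeft and LookRight slide the camera between slots with wraparound, while ChangeAmountDisplayed applies the focused slot's item visibility.
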(event `self.ReceiveBeginPlay`
  (bind _item_slots (`self.Item Slots`))
  ; Add Camera Look and location spots
  (bind _asbp_player (cast `/Game/MatthewTest/Player/BP_Player` (`GameplayStatics.GetPlayerCharacter` 0)))
  (set `self.Player` _asbp_player)
  (for _array_element (`self.GetComponentsByTag` "/Script/Engine.SceneComponent" "Items")
    (`BlueprintMapLibrary.Map_Add` _item_slots _array_element (make `/Game/MatthewTest/Enums/ShelfItemSlot` null)))
  (bind _keys (`BlueprintMapLibrary.Map_Keys` _item_slots))
  (for _array_element_2 _keys
    (bind _asscene_component (cast `SceneComponent` _array_element_2))
    (bind _output_get (set `self.CurItemSlotTransform` (`SceneComponent.GetRelativeTransform` _asscene_component)))
    (bind _returnvalue (`AddComponent|NODE_AddSceneComponent-0`))
    (`SceneComponent.K2_AttachToComponent` _returnvalue _asscene_component "None" "SnapToTarget" "KeepRelative" "KeepRelative" true)
    (`SceneComponent.K2_SetRelativeTransform` _returnvalue (`KismetMathLibrary.MakeTransform` (`self.LookPointOffset`) (.rotation _output_get) (.scale _output_get)) false false)
    (`KismetArrayLibrary.Array_Add` (`self.ItemLookPoints`) _returnvalue)
    (bind _returnvalue_2 (`AddComponent|NODE_AddSceneComponent-1`))
    (`SceneComponent.K2_AttachToComponent` _returnvalue_2 _asscene_component "None" "SnapToTarget" "KeepRelative" "KeepRelative" true)
    (`SceneComponent.K2_SetRelativeTransform` _returnvalue_2 (`KismetMathLibrary.MakeTransform` (`self.CameraPointOffset`) (.rotation _output_get) (.scale _output_get)) false false)
    (`KismetArrayLibrary.Array_Add` (`self.ItemCameraPoints`) _returnvalue_2)))

(event `ChangeAmountDisplayed`
  (bind _output_get (set `self.TempIntMap` (`.ItemRefs_11_23701C7546586C4E98784CA399694FE8` (break `/Game/MatthewTest/Enums/ShelfItemSlot` (`.Value` (`BlueprintMapLibrary.Map_GetKeyValueByIndex` (`self.Item Slots`) (`self.CurFocusedSlot`)))))))
  (bind (_keypin _valuepin) (`|MapForEach` _output_get)
    (:`then`
      (`self.SetActorHiddenInGame` _keypin _valuepin))))

(event `/Game/Structure/IE_Interactable.Interact`
  (bind _player (`self.Player`))
  (bind _camera (`/Game/MatthewTest/Player/BP_Player.Camera` _player))
  (bind _playercontroller (`/Game/MatthewTest/Player/BP_Player.PlayerController` _player))
  (bind _returnvalue (`SceneComponent.K2_GetComponentLocation` (`|GetArrayItem` (`self.ItemCameraPoints`))))
  (`/Game/MatthewTest/Player/BP_Player.RemoveMappings` _player)
  (set `self.OriginalCamRotation` (`SceneComponent.K2_GetComponentRotation` _camera))
  (set `CameraComponent.bUsePawnControlRotation` false _camera)
  (`TimelineComponent.SetPlayRate` (`self.CameraMovement`) (/ 1.0 (`self.CameraMoveTime`)))
  (bind (_direction _newtrack_0) (`Timeline|CameraMovement` :!via `PlayFromStart`)
    (:`Update`
      (`SceneComponent.K2_SetWorldLocationAndRotation` _camera (`KismetMathLibrary.VLerp` (`SceneComponent.K2_GetComponentLocation` (`/Game/MatthewTest/Player/BP_Player.CameraDefaultLocation` _player)) _returnvalue _newtrack_0) (`KismetMathLibrary.RLerp` (`self.OriginalCamRotation`) (`KismetMathLibrary.FindLookAtRotation` _returnvalue (`SceneComponent.K2_GetComponentLocation` (`|GetArrayItem` (`self.ItemLookPoints`)))) _newtrack_0) false false))
    (:`Finished`
      (set `PlayerController.bShowMouseCursor` true _playercontroller)
      (`EnhancedInputSubsystemInterface.AddMappingContext` (pcsubsystem `EnhancedInputLocalPlayerSubsystem` _playercontroller) "/Game/MatthewTest/Player/ShelfMapping/IMC_Shelving.IMC_Shelving" 0 (struct))
      (set `self.CurFocusedSlot` 0)
      (bind _returnvalue_2 (`|CreateWidget` "/Game/MatthewTest/Interactables/UW_Shelf.UW_Shelf_C"))
      (`UserWidget.AddToViewport` _returnvalue_2 0))))

(event `LookLeft`
  (bind _itemcamerapoints (`self.ItemCameraPoints`))
  (bind _curfocusedslot (`self.CurFocusedSlot`))
  (bind _returnvalue (- _curfocusedslot 1))
  (bind _camera (`/Game/MatthewTest/Player/BP_Player.Camera` (`self.Player`)))
  (bind _returnvalue_2 (`SceneComponent.K2_GetComponentLocation` (`|GetArrayItem` _itemcamerapoints _curfocusedslot)))
  (bind _returnvalue_3 (- (`KismetArrayLibrary.Array_Length` _itemcamerapoints) 1))
  ; Camera Left and Right Slots
  (if (not (`self.IsMoving`))
    (set `self.IsMoving` true)
    (if (< _returnvalue 0)
      (set `self.NegativeChecker` true)
      (else
        (set `self.NegativeChecker` false)))
    (`TimelineComponent.SetPlayRate` (`self.CameraMovementItems`) (/ 1.0 (`self.CameraMoveTimeItems`)))
    (bind (_direction _newtrack_0) (`Timeline|CameraMovementItems` :!via `PlayFromStart`)
      (:`Update`
        (if (`self.NegativeChecker`)
          (`SceneComponent.K2_SetWorldLocation` _camera (`KismetMathLibrary.VLerp` _returnvalue_2 (`SceneComponent.K2_GetComponentLocation` (`|GetArrayItem` _itemcamerapoints _returnvalue_3)) _newtrack_0) false false)
          (else
            (`SceneComponent.K2_SetWorldLocation` _camera (`KismetMathLibrary.VLerp` _returnvalue_2 (`SceneComponent.K2_GetComponentLocation` (`|GetArrayItem` _itemcamerapoints _returnvalue)) _newtrack_0) false false))))
      (:`Finished`
        (if (`self.NegativeChecker`)
          (set `self.CurFocusedSlot` _returnvalue_3)
          (else
            (set `self.CurFocusedSlot` _returnvalue)))
        (set `self.IsMoving` false)))))

(event `LookRight`
  (bind _itemcamerapoints (`self.ItemCameraPoints`))
  (bind _curfocusedslot (`self.CurFocusedSlot`))
  (bind _returnvalue (mod (+ _curfocusedslot 1) (`KismetArrayLibrary.Array_Length` _itemcamerapoints)))
  ; Camera Left and Right Slots
  (if (not (`self.IsMoving`))
    ;; Can make swoop in take more or less time
    (set `self.IsMoving` true)
    (`TimelineComponent.SetPlayRate` (`self.CameraMovementItems2`) (/ 1.0 (`self.CameraMoveTimeItems`)))
    (bind (_direction _newtrack_0) (`Timeline|CameraMovementItems2` :!via `PlayFromStart`)
      (:`Update`
        (`SceneComponent.K2_SetWorldLocation` (`/Game/MatthewTest/Player/BP_Player.Camera` (`self.Player`)) (`KismetMathLibrary.VLerp` (`SceneComponent.K2_GetComponentLocation` (`|GetArrayItem` _itemcamerapoints _curfocusedslot)) (`SceneComponent.K2_GetComponentLocation` (`|GetArrayItem` _itemcamerapoints _returnvalue)) _newtrack_0) false false))
      (:`Finished`
        (set `self.CurFocusedSlot` _returnvalue)
        (set `self.IsMoving` false)))))

(fn `UserConstructionScript`)