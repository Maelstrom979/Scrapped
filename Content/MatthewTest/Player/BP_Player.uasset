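; First-person player character for a shop-style game with movement, interaction, a class-to-count inventory and money-checked purchasing.
; A camera sphere trace messages interactables; shelves receive left/right slot input, and leaving focus uses a timeline to restore the camera.
; Enhanced Input contexts and input modes swap between gameplay and the animated inventory, while cursor traces move or collect world items.
; BP_GameInstance runs the calendar and records purchases, alongside debug test keys.
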(event `EnhancedInput|/Game/MatthewTest/Player/IA_Jump`
  (params (ActionValue :type Boolean) (ElapsedSeconds :type "Float (double-precision)") (TriggeredSeconds :type "Float (double-precision)") (InputAction :type "InputAction Object Reference" :default "/Game/MatthewTest/Player/IA_Jump.IA_Jump"))
  ; Simple Movement
  (:`Triggered`
    (`self.Jump`)))

(event `EnhancedInput|/Game/MatthewTest/Player/IA_Look`
  (params (ActionValue :type "Vector2D Structure") (ElapsedSeconds :type "Float (double-precision)") (TriggeredSeconds :type "Float (double-precision)") (InputAction :type "InputAction Object Reference" :default "/Game/MatthewTest/Player/IA_Look.IA_Look"))
  ; Simple Movement
  (:`Triggered`
    (`self.Look` ActionValue_X ActionValue_Y)))

(event `EnhancedInput|/Game/MatthewTest/Player/IA_WalkBackward`
  (params (ActionValue :type Boolean) (ElapsedSeconds :type "Float (double-precision)") (TriggeredSeconds :type "Float (double-precision)") (InputAction :type "InputAction Object Reference" :default "/Game/MatthewTest/Player/IA_WalkBackward.IA_WalkBackward"))
  (bind (_returnvalue_roll _returnvalue_pitch _returnvalue_yaw) (`KismetMathLibrary.BreakRotator` (`self.GetControlRotation`)))
  ; Simple Movement
  (:`Triggered`
    (`self.AddMovementInput` (`KismetMathLibrary.Normal` (`KismetMathLibrary.GetForwardVector` (`KismetMathLibrary.MakeRotator` _returnvalue_roll 0.0 _returnvalue_yaw))) (* (`self.Speed`) -1.0))))

(event `EnhancedInput|/Game/MatthewTest/Player/IA_WalkForward`
  (params (ActionValue :type Boolean) (ElapsedSeconds :type "Float (double-precision)") (TriggeredSeconds :type "Float (double-precision)") (InputAction :type "InputAction Object Reference" :default "/Game/MatthewTest/Player/IA_WalkForward.IA_WalkForward"))
  (bind (_returnvalue_roll _returnvalue_pitch _returnvalue_yaw) (`KismetMathLibrary.BreakRotator` (`self.GetControlRotation`)))
  ; Simple Movement
  (:`Triggered`
    (`self.AddMovementInput` (`KismetMathLibrary.Normal` (`KismetMathLibrary.GetForwardVector` (`KismetMathLibrary.MakeRotator` _returnvalue_roll 0.0 _returnvalue_yaw))) (`self.Speed`))))

(event `EnhancedInput|/Game/MatthewTest/Player/IA_WalkRight`
  (params (ActionValue :type Boolean) (ElapsedSeconds :type "Float (double-precision)") (TriggeredSeconds :type "Float (double-precision)") (InputAction :type "InputAction Object Reference" :default "/Game/MatthewTest/Player/IA_WalkRight.IA_WalkRight"))
  (bind (_returnvalue_roll _returnvalue_pitch _returnvalue_yaw) (`KismetMathLibrary.BreakRotator` (`self.GetControlRotation`)))
  ; Simple Movement
  (:`Triggered`
    (`self.AddMovementInput` (`KismetMathLibrary.Normal` (`KismetMathLibrary.GetRightVector` (`KismetMathLibrary.MakeRotator` 0.0 0.0 _returnvalue_yaw))) (`self.Speed`))))

(event `EnhancedInput|/Game/MatthewTest/Player/IA_WalkLeft`
  (params (ActionValue :type Boolean) (ElapsedSeconds :type "Float (double-precision)") (TriggeredSeconds :type "Float (double-precision)") (InputAction :type "InputAction Object Reference" :default "/Game/MatthewTest/Player/IA_WalkLeft.IA_WalkLeft"))
  (bind (_returnvalue_roll _returnvalue_pitch _returnvalue_yaw) (`KismetMathLibrary.BreakRotator` (`self.GetControlRotation`)))
  ; Simple Movement
  (:`Triggered`
    (`self.AddMovementInput` (`KismetMathLibrary.Normal` (`KismetMathLibrary.GetRightVector` (`KismetMathLibrary.MakeRotator` 0.0 0.0 _returnvalue_yaw))) (* (`self.Speed`) -1.0))))

(event `self.ReceiveBeginPlay`
  ; Code for setting input mapping context
  (bind _asbp_player_controller (cast `/Game/MatthewTest/Player/BP_PlayerController` (`GameplayStatics.GetPlayerController` 0)))
  (bind _output_get (set `self.PlayerController` _asbp_player_controller))
  (`EnhancedInputSubsystemInterface.AddMappingContext` (pcsubsystem `EnhancedInputLocalPlayerSubsystem` _output_get) "/Game/MatthewTest/Player/IMC_CharacterMovement.IMC_CharacterMovement" 0 (struct))
  (bind _asbp_game_instance (cast `/Game/MatthewTest/BP_GameInstance` (`GameplayStatics.GetGameInstance`)))
  (bind _output_get_2 (set `self.Game Instance` _asbp_game_instance))
  (`/Game/MatthewTest/BP_GameInstance.StartGameCalendar` _output_get_2)
  (`self.RemoveNonPermWidgets`))

(event `EnhancedInput|/Game/MatthewTest/Player/IA_Interact`
  (params (ActionValue :type Boolean) (ElapsedSeconds :type "Float (double-precision)") (TriggeredSeconds :type "Float (double-precision)") (InputAction :type "InputAction Object Reference" :default "/Game/MatthewTest/Player/IA_Interact.IA_Interact"))
  (bind _camera (`self.Camera`))
  (bind _returnvalue (`SceneComponent.K2_GetComponentLocation` _camera))
  (:`Triggered`
    (if (not (`self.InvIsOpen`))
      (set `self.OriginalCamRot` (`SceneComponent.K2_GetComponentRotation` _camera))
      (bind _outhit (`KismetSystemLibrary.SphereTraceSingle` :`Start` _returnvalue :`End` (+ _returnvalue (* (`SceneComponent.GetForwardVector` _camera) (`self.SphereTraceDistance`))) :`Radius` (`self.SphereTraceSize`) :`TraceChannel` "TraceTypeQuery1" :`bTraceComplex` true :`DrawDebugType` "ForDuration"))
      (bind _output_get (set `self.InteractingActor` (`.HitActor` (`GameplayStatics.BreakHitResult` _outhit))))
      (if (`KismetSystemLibrary.DoesImplementInterface` _output_get "/Game/Structure/IE_Interactable.IE_Interactable_C")
        (message `/Game/Structure/IE_Interactable.Interact` _output_get)))))

(event `EnhancedInput|/Game/MatthewTest/Player/ShelfMapping/IA_LeftSlot`
  (params (ActionValue :type Boolean) (ElapsedSeconds :type "Float (double-precision)") (TriggeredSeconds :type "Float (double-precision)") (InputAction :type "InputAction Object Reference" :default "/Game/MatthewTest/Player/ShelfMapping/IA_LeftSlot.IA_LeftSlot"))
  ; Shelving
  (:`Triggered`
    (`self.GoLeft`)))

(event `GoLeft`
  ; Shelving
  (bind _asbp_base_shelf (cast `/Game/MatthewTest/Interactables/BP_BaseShelf` (`self.InteractingActor`)))
  (`/Game/MatthewTest/Interactables/BP_BaseShelf.LookLeft` _asbp_base_shelf))

(event `EnhancedInput|/Game/MatthewTest/Player/IA_OpenInventory`
  (params (ActionValue :type Boolean) (ElapsedSeconds :type "Float (double-precision)") (TriggeredSeconds :type "Float (double-precision)") (InputAction :type "InputAction Object Reference" :default "/Game/MatthewTest/Player/IA_OpenInventory.IA_OpenInventory"))
  (:`Triggered`
    (`self.OpenInventory`)))

(event `EnhancedInput|/Game/MatthewTest/Player/ShelfMapping/IA_RightSlot`
  (params (ActionValue :type Boolean) (ElapsedSeconds :type "Float (double-precision)") (TriggeredSeconds :type "Float (double-precision)") (InputAction :type "InputAction Object Reference" :default "/Game/MatthewTest/Player/ShelfMapping/IA_RightSlot.IA_RightSlot"))
  ; Shelving
  (:`Triggered`
    (`self.GoRight`)))

(event `OpenInventory`
  (bind _invwidget (`self.INVWidget`))
  (bind _playercontroller (`self.PlayerController`))
  (`self.RemoveMappings`)
  (if (`self.InvIsOpen`)
    (bind _asuw_inventory (cast `/Game/MatthewTest/Player/UW_Inventory` _invwidget))
    (`/Game/MatthewTest/Player/UW_Inventory.Animation Off Screen` _asuw_inventory)
    ; Time Of Inventory Animation, Change Delay if speed changes
    (`KismetSystemLibrary.Delay` (`self.InventoryCloseTime`))
    (`Widget.RemoveFromParent` _invwidget)
    (`self.AddPlayerMappings`)
    (set `self.InvIsOpen` false)
    (else
      (`UserWidget.AddToViewport` _invwidget 0)
      (bind _asuw_inventory_2 (cast `/Game/MatthewTest/Player/UW_Inventory` _invwidget))
      (`/Game/MatthewTest/Player/UW_Inventory.Animation Onto Screen` _asuw_inventory_2)
      (`EnhancedInputSubsystemInterface.AddMappingContext` (pcsubsystem `EnhancedInputLocalPlayerSubsystem` _playercontroller) "/Game/MatthewTest/Player/IMC_Inventory.IMC_Inventory" 0 (struct))
      (set `PlayerController.bShowMouseCursor` true _playercontroller)
      (`WidgetBlueprintLibrary.SetInputMode_GameAndUIEx` _playercontroller null "DoNotLock" false)
      (set `self.InvIsOpen` true))))

(event `GoRight`
  ; Shelving
  (bind _asbp_base_shelf (cast `/Game/MatthewTest/Interactables/BP_BaseShelf` (`self.InteractingActor`)))
  (`/Game/MatthewTest/Interactables/BP_BaseShelf.LookRight` _asbp_base_shelf))

(event `EnhancedInput|/Game/MatthewTest/Player/IA_LeaveFocus`
  (params (ActionValue :type Boolean) (ElapsedSeconds :type "Float (double-precision)") (TriggeredSeconds :type "Float (double-precision)") (InputAction :type "InputAction Object Reference" :default "/Game/MatthewTest/Player/IA_LeaveFocus.IA_LeaveFocus"))
  (bind _camera (`self.Camera`))
  (:`Triggered`
    (bind _asbp_laptop (cast `/Game/MatthewTest/Interactables/BP_Laptop` (`self.InteractingActor`))
      (:`then`
        (`/Game/MatthewTest/Interactables/BP_Laptop.SetScreen` _asbp_laptop null))
      (:`CastFailed`
        _))
    (set `PlayerController.bShowMouseCursor` false (`self.PlayerController`))
    (`self.RemoveMappings`)
    (`self.RemoveNonPermWidgets`)
    (set `self.InteractingActor` null)
    (bind _output_get (set `self.OffsetStartCamLocation` (`SceneComponent.K2_GetComponentLocation` _camera)))
    (bind _output_get_2 (set `self.OffsetStartCamRotation` (`SceneComponent.K2_GetComponentRotation` _camera)))
    (`TimelineComponent.SetPlayRate` (`self.ReturnCameraPosition`) (/ 1.0 (`self.CameraMoveTime`)))
    (bind (_direction _newtrack_0) (`Timeline|ReturnCameraPosition` :!via `PlayFromStart`)
      (:`Update`
        (`SceneComponent.K2_SetWorldLocationAndRotation` (`self.Camera`) (`KismetMathLibrary.VLerp` _output_get (`SceneComponent.K2_GetComponentLocation` (`self.CameraDefaultLocation`)) _newtrack_0) (`KismetMathLibrary.RLerp` _output_get_2 (`self.OriginalCamRot`) _newtrack_0) false false))
      (:`Finished`
        (`self.AddPlayerMappings`)
        (set `CameraComponent.bUsePawnControlRotation` true _camera)
        (`WidgetBlueprintLibrary.SetInputMode_GameOnly` (`self.PlayerController`))))))

(event `CheckToRemoveItem`
  (params (ItemToCheck :type "/Game/AceTest/Draftdumpster/BP_ParentItem Class Reference"))
  (bind _inventory (`self.Inventory`))
  (if (<= (`BlueprintMapLibrary.Map_Find` _inventory ItemToCheck) 0)
    (`BlueprintMapLibrary.Map_Remove` _inventory ItemToCheck)))

(event `RemoveNonPermWidgets`
  ;[0 0 0 0.5] Call these when changing forms
  (`WidgetLayoutLibrary.RemoveAllWidgets`)
  (for _array_element (`self.PermanentWidgets`)
    (`UserWidget.AddToViewport` _array_element 0)))

(event `RemoveMappings`
  (bind _playercontroller (`self.PlayerController`))
  ;[0 0 0 0.5] Call these when changing forms
  (`EnhancedInputSubsystemInterface.ClearAllMappings` (pcsubsystem `EnhancedInputLocalPlayerSubsystem` _playercontroller))
  (`EnhancedInputLibrary.FlushPlayerInput` _playercontroller))

(event `EnhancedInput|/Game/AceTest/inputs/IA_LeftHold`
  (params (ActionValue :type Boolean) (ElapsedSeconds :type "Float (double-precision)") (TriggeredSeconds :type "Float (double-precision)") (InputAction :type "InputAction Object Reference" :default "/Game/AceTest/inputs/IA_LeftHold.IA_LeftHold"))
  (bind _returnvalue (`GameplayStatics.GetPlayerController` 0))
  (bind (_locationx _locationy) (`PlayerController.GetMousePosition` _returnvalue))
  (bind (_worldposition _worlddirection) (`GameplayStatics.DeprojectScreenToWorld` _returnvalue (`KismetMathLibrary.MakeVector2D` _locationx _locationy)))
  (:`Triggered`
    (bind _outhit (`KismetSystemLibrary.LineTraceSingle` :`Start` _worldposition :`End` (* _worlddirection 5000.0) :`TraceChannel` "TraceTypeQuery1" :`bTraceComplex` true :`DrawDebugType` "Persistent"))
    (if (!= (`GameplayStatics.GetObjectClass` (`.HitActor` (`GameplayStatics.BreakHitResult` _outhit))) "/Game/AceTest/BP_Dumpster.BP_Dumpster_C")
      (`self.K2_SetActorLocation` (`.HitActor` (`GameplayStatics.BreakHitResult` _outhit)) (`KismetMathLibrary.MakeVector` (.x (`.Location` (`GameplayStatics.BreakHitResult` _outhit))) (.y (`.Location` (`GameplayStatics.BreakHitResult` _outhit)))) false false))))

(event `AddPlayerMappings`
  (bind _playercontroller (`self.PlayerController`))
  ;[0 0 0 0.5] Call these when changing forms
  (for _array_element (`self.PermanentMappings`)
    (`EnhancedInputSubsystemInterface.AddMappingContext` (pcsubsystem `EnhancedInputLocalPlayerSubsystem` _playercontroller) _array_element 0 (struct))
    (`WidgetBlueprintLibrary.SetInputMode_GameOnly` _playercontroller)
    (set `PlayerController.bShowMouseCursor` false _playercontroller)))

(event `Key|Q`
  (params (Key :type "Key Structure"))
  ; Testing Game Instance Functions
  (:`Pressed`
    (`/Game/MatthewTest/BP_GameInstance.NextDay` (`self.Game Instance`))))

(event `EnhancedInput|/Game/AceTest/inputs/IA_Click`
  (params (ActionValue :type Boolean) (ElapsedSeconds :type "Float (double-precision)") (TriggeredSeconds :type "Float (double-precision)") (InputAction :type "InputAction Object Reference" :default "/Game/AceTest/inputs/IA_Click.IA_Click"))
  (bind _hitresult (`PlayerController.GetHitResultUnderCursorByChannel` (`PlayerState.GetPlayerController` (`GameplayStatics.GetPlayerState` 0)) "TraceTypeQuery1" true))
  ; Code to add objects into inventory
  (:`Triggered`
    (if (!= (`GameplayStatics.GetObjectClass` (`.HitActor` (`GameplayStatics.BreakHitResult` _hitresult))) "/Game/AceTest/BP_Dumpster.BP_Dumpster_C")
      (bind _asbp_parent_item (castclass `/Game/AceTest/Draftdumpster/BP_ParentItem` (`GameplayStatics.GetObjectClass` (`.HitActor` (`GameplayStatics.BreakHitResult` _hitresult)))))
      (`self.AddToInventory` _asbp_parent_item 1)
      (`self.K2_DestroyActor` (`.HitActor` (`GameplayStatics.BreakHitResult` _hitresult))))))

(event `Key|One`
  (params (Key :type "Key Structure"))
  ; Testing Game Instance Functions
  (:`Pressed`
    (`KismetSystemLibrary.PrintString` (`|GetEnumeratorNameAsString` (`/Game/MatthewTest/BP_GameInstance.Day Of Week` (`self.Game Instance`))))))

(event `Key|Two`
  (params (Key :type "Key Structure"))
  ; Testing Game Instance Functions
  (:`Pressed`
    (`KismetSystemLibrary.PrintString` (`|GetEnumeratorNameAsString` (`/Game/MatthewTest/BP_GameInstance.Month` (`self.Game Instance`))))))

(event `Key|Three`
  (params (Key :type "Key Structure"))
  ; Testing Game Instance Functions
  (:`Pressed`
    (`KismetSystemLibrary.PrintString` (`KismetStringLibrary.Conv_IntToString` (`/Game/MatthewTest/BP_GameInstance.DayOfMonth` (`self.Game Instance`))))))

(event `Key|E`
  (params (Key :type "Key Structure"))
  (bind _maptest (`self.MapTest`))
  (bind (_key _value) (`BlueprintMapLibrary.Map_GetKeyValueByIndex` (`self.MapTest`)))
  (bind (_key_2 _value_2) (`BlueprintMapLibrary.Map_GetKeyValueByIndex` _maptest))
  ; Check the inventory
  (:`Pressed`
    (bind _outactors (`GameplayStatics.GetAllActorsOfClass` "/Game/AceTest/Draftdumpster/Common/BP_Clock.BP_Clock_C"))
    (bind _output_get (set `self.Temp internal Map Copy` (`.ItemRefs_11_23701C7546586C4E98784CA399694FE8` (break `/Game/MatthewTest/Enums/ShelfItemSlot` _value_2))))
    (for _index (range (`.HowMany_5_907D4EAC4C44BDD81D7D7BBC4B7E3AA1` (break `/Game/MatthewTest/Enums/ShelfItemSlot` _value_2)))
      (bind _asbp_parent_item (cast `/Game/AceTest/Draftdumpster/BP_ParentItem` (`|GetArrayItem` _outactors _index)))
      (`BlueprintMapLibrary.Map_Add` _output_get _asbp_parent_item true))
    (`BlueprintMapLibrary.Map_Add` _maptest _key (make `/Game/MatthewTest/Enums/ShelfItemSlot` (break `/Game/MatthewTest/Enums/ShelfItemSlot` _value) (`.HowMany_5_907D4EAC4C44BDD81D7D7BBC4B7E3AA1` (break `/Game/MatthewTest/Enums/ShelfItemSlot` _value)) _output_get))))

(event `Purchase`
  (params (Price :type "Float (double-precision)") (Object :type "/Game/AceTest/Draftdumpster/BP_ParentItem Class Reference") (Amount :type Integer))
  (bind _returnvalue (* Price Amount))
  (bind _inventory (`self.Inventory`))
  (bind (_value _returnvalue_2) (`BlueprintMapLibrary.Map_Find` _inventory Object))
  ; Event to buy an item, takes amount, item's class, and price
  (if (>= (`self.Money`) _returnvalue)
    (if _returnvalue_2
      (`BlueprintMapLibrary.Map_Add` _inventory Object (+ _value Amount))
      (set `self.Money` (- (`self.Money`) _returnvalue) :!label _label)
      (`/Game/MatthewTest/BP_GameInstance.PurchaseItem` (`self.Game Instance`) Object Amount)
      (elif (< (`BlueprintMapLibrary.Map_Length` _inventory) (`self.InventoryMaxSize`))
        (`BlueprintMapLibrary.Map_Add` _inventory Object Amount)
        (goto _label)
        (else
          (`KismetSystemLibrary.PrintString` "InvFull"))))
    (else
      (`KismetSystemLibrary.PrintString` "Too Poor"))))

(event `AddToInventory`
  (params (ItemToAdd :type "/Game/AceTest/Draftdumpster/BP_ParentItem Class Reference") (HowMany :type Integer))
  (bind _inventory (`self.Inventory`))
  (bind (_value _returnvalue) (`BlueprintMapLibrary.Map_Find` _inventory ItemToAdd))
  ; If the item is already in the inventory then add however many are being added to the total, otherwise set the current amount to that value
  (if _returnvalue
    (`BlueprintMapLibrary.Map_Add` _inventory ItemToAdd (+ _value HowMany))
    (else
      (`BlueprintMapLibrary.Map_Add` _inventory ItemToAdd HowMany))))

(fn `Look`
  (params (`Action x` :type "Float (double-precision)") (`Action Y` :type "Float (double-precision)"))
  ; Look function
  (`self.AddControllerYawInput` `Action x`)
  (`self.AddControllerPitchInput` (* `Action Y` -1.0)))

(fn `Movement`)

(fn `UserConstructionScript`)