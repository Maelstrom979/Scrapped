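; Dumpster interactable that, while stocked, starts a one-time dumpster-diving view with loot buried in trash.
; Interacting rolls rarity-tiered items from Common to Legendary, then spawns them among a large BP_Trash pile at random points inside the TrashSpawn box.
; A timeline swoops the player's camera to CameraPoint facing ViewPoint, then enables the cursor and dumpster-diving input mapping.
; It also shows WBP_Dumpster and clears Stocked.
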(event `self.ReceiveBeginPlay`
  (bind _asbp_player (cast `/Game/MatthewTest/Player/BP_Player` (`GameplayStatics.GetPlayerCharacter` 0)))
  (set `self.As BP Player` _asbp_player))

(event `/Game/Structure/IE_Interactable.Interact`
  (bind _as_bp_player (`self.As BP Player`))
  (bind _as_bp_player_2 (`self.As BP Player`))
  (bind _returnvalue (`SceneComponent.K2_GetComponentLocation` (`self.CameraPoint`)))
  (bind _camera (`/Game/MatthewTest/Player/BP_Player.Camera` _as_bp_player_2))
  (bind _playercontroller (`/Game/MatthewTest/Player/BP_Player.PlayerController` _as_bp_player))
  (if (`self.Stocked`)
    (`|ExecutionSequence`
      (:`then_0`
        (`self.ItemsThatSpawn`))
      (:`then_1`
        (`self.SpawnTrash`))
      (:`then_2`
        (`/Game/MatthewTest/Player/BP_Player.RemoveMappings` _as_bp_player)
        (set `self.NewVar` (`SceneComponent.K2_GetComponentRotation` _camera))
        ; Can make swoop in take more or less time
        (set `CameraComponent.bUsePawnControlRotation` false _camera)
        (`TimelineComponent.SetPlayRate` (`self.graphtime`) (/ 1.0 (`self.NewVar_0`)))
        (bind (_direction _newtrack_0) (`Timeline|graphtime`)
          (:`Update`
            (`SceneComponent.K2_SetWorldLocationAndRotation` _camera (`KismetMathLibrary.VLerp` (`SceneComponent.K2_GetComponentLocation` (`/Game/MatthewTest/Player/BP_Player.CameraDefaultLocation` _as_bp_player_2)) _returnvalue _newtrack_0) (`KismetMathLibrary.RLerp` (`self.NewVar`) (`KismetMathLibrary.FindLookAtRotation` _returnvalue (`SceneComponent.K2_GetComponentLocation` (`self.ViewPoint`))) _newtrack_0) false false))
          (:`Finished`
            (set `PlayerController.bShowMouseCursor` true _playercontroller)
            (`EnhancedInputSubsystemInterface.AddMappingContext` (pcsubsystem `EnhancedInputLocalPlayerSubsystem` _playercontroller) "/Game/AceTest/inputs/IMC_Dumpsterdiving.IMC_Dumpsterdiving" 0 (struct))
            (`WidgetBlueprintLibrary.SetInputMode_GameAndUIEx` _playercontroller null "DoNotLock" false true))))
      (:`then_3`
        (bind _returnvalue_2 (`|CreateWidget` "/Game/AceTest/UI/WBP_Dumpster.WBP_Dumpster_C"))
        (`UserWidget.AddToViewport` _returnvalue_2 0)
        (set `self.Stocked` false)))))

(fn `ChanceMaker`
  (returns (NewParam :type String))
  (bind _returnvalue (`KismetMathLibrary.RandomIntegerInRange` 1 100))
  (if (>= _returnvalue 97)
    (return "legendary")
    (elif (>= _returnvalue 80)
      (return "Rare")
      (elif (>= _returnvalue 60)
        (return "Uncommon")
        (else
          (return "Common"))))))

(fn `ItemsThatSpawn`
  (bind _spawneditems (`self.SpawnedItems`))
  (bind _output_get (set `self.NewVar_1` (`KismetMathLibrary.RandomIntegerInRange` 6 9)))
  (for _index (range (+ _output_get 1))
    (bind _newparam (`self.ChanceMaker`))
    ; Determines what items are spawned
    (switch `string` _newparam
      (:`Common`
        (`KismetArrayLibrary.Array_Set` _spawneditems _index (`KismetArrayLibrary.Array_Random` (`self.CommonItems`))))
      (:`Uncommon`
        (`KismetArrayLibrary.Array_Set` _spawneditems _index (`KismetArrayLibrary.Array_Random` (`self.UncommonItems`))))
      (:`Rare`
        (`KismetArrayLibrary.Array_Set` _spawneditems _index (`KismetArrayLibrary.Array_Random` (`self.Rareitems`))))
      (:`Legendary`
        (`KismetArrayLibrary.Array_Set` _spawneditems _index (`KismetArrayLibrary.Array_Random` (`self.Legendary`)))))))

(fn `SpawnItems`)

(fn `SpawnTrash`
  (locals (Trash_grp :type "Array of /Game/AceTest/BP_Trash Object Reference"))
  (bind _trashspawn (`self.TrashSpawn`))
  (bind _trashspawn_2 (`self.TrashSpawn`))
  (`|ExecutionSequence`
    (:`then_0`
      ; Spawn TrashPile
      (for _ (range 116)
        (bind _returnvalue (`|SpawnActorFromClass` "/Game/AceTest/BP_Trash.BP_Trash_C" (`KismetMathLibrary.MakeTransform` (`KismetMathLibrary.RandomPointInBoundingBox` (`SceneComponent.K2_GetComponentLocation` _trashspawn_2) (`BoxComponent.GetScaledBoxExtent` _trashspawn_2)) (`KismetMathLibrary.RandomRotator` true)) "AdjustIfPossibleButAlwaysSpawn" "MultiplyWithRoot" null null))
        (`KismetArrayLibrary.Array_Add` (`local.Trash_grp`) _returnvalue)))
    (:`then_1`
      ; Spawn Items
      (for _index (range (+ (`self.NewVar_1`) 1))
        (`|SpawnActorFromClass` (`|GetArrayItem` (`self.SpawnedItems`) _index) (`KismetMathLibrary.MakeTransform` (`KismetMathLibrary.RandomPointInBoundingBox` (`SceneComponent.K2_GetComponentLocation` _trashspawn) (`BoxComponent.GetScaledBoxExtent` _trashspawn)) (`KismetMathLibrary.RandomRotator` true)) "AdjustIfPossibleButAlwaysSpawn" "MultiplyWithRoot" null null)))))

(fn `UserConstructionScript`)