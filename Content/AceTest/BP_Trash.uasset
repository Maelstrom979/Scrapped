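; BP_Trash is a trash object that takes on a random shape when play begins.
; On BeginPlay, SwitchForms picks Cylinder, Cube or Cone through a random integer, and the result replaces the static mesh on the Sphere component.
; An author note indicates that models for these forms are still to be made, and the construction script is empty.
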(event `self.ReceiveBeginPlay`
  (bind _newparam (`self.SwitchForms`))
  (`StaticMeshComponent.SetStaticMesh` (`self.Sphere`) _newparam))

(fn `SwitchForms`
  (returns (NewParam :type "StaticMesh Object Reference"))
  (locals (NewLocalVar :type "StaticMesh Object Reference"))
  ; Chance for the form to change // make modesl for them to change into
  (switch `int` (`KismetMathLibrary.RandomIntegerInRange` 1 3)
    (:`1`
      (bind _output_get (set `local.NewLocalVar` "/Engine/EngineMeshes/Cylinder.Cylinder"))
      (return _output_get))
    (:`2`
      (bind _output_get_2 (set `local.NewLocalVar` "/Engine/BasicShapes/Cube.Cube"))
      (return _output_get_2))
    (:`3`
      (bind _output_get_3 (set `local.NewLocalVar` "/Engine/BasicShapes/Cone.Cone"))
      (return _output_get_3))))

(fn `UserConstructionScript`)